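; Player controller that creates the game HUD and spawns numbered button widgets into it.
; BeginPlay adds the HUD to the viewport, flips its HumanBox 180 degrees and binds the SpawnButton event.
; Each spawn numbers a rotated button from an incrementing, externally settable Count.
; BP_Manager's IsBotPlayed flag routes the button to HumanBox when true, otherwise to BotBox.
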(event `self.ReceiveBeginPlay`
  (`parent.ReceiveBeginPlay`)
  (bind _returnvalue (`|CreateWidget` "/Game/UI/Game/HUD.HUD_C" self))
  (`UserWidget.AddToViewport` _returnvalue 0)
  (`Widget.SetRenderTransformAngle` (`/Game/UI/Game/HUD.HumanBox` _returnvalue) 180.0)
  (add `self.SpawnButtonEvent` (delegate `SpawnButton_Event`)))

(event `SpawnButton_Event`
  (bind _returnvalue (`|CreateWidget` "/Game/UI/Game/Button.Button_C"))
  (bind _result (`/Engine/EditorBlueprintResources/StandardMacros.IncrementInt` (`self.Count`))
    (:`  `
      (`/Game/UI/Game/Button.SetButtonValue` _returnvalue _result)
      (`UserWidget.SetPadding` _returnvalue (`self.Padding`))
      (`Widget.SetRenderTransformAngle` _returnvalue 180.0)
      (bind _returnvalue_2 (`GameplayStatics.GetActorOfClass` "/Game/Blueprints/Game/BP_Manager.BP_Manager_C"))
      (bind _returnvalue_3 (`ManagePiece.GetIsBotPlayed` _returnvalue_2))
      (if _returnvalue_3
        (`VerticalBox.AddChildToVerticalBox` (`/Game/UI/Game/HUD.HumanBox` (stale `self.ReceiveBeginPlay` _returnvalue)) _returnvalue)
        (else
          (`VerticalBox.AddChildToVerticalBox` (`/Game/UI/Game/HUD.BotBox` (stale `self.ReceiveBeginPlay` _returnvalue)) _returnvalue))))))

(fn `SetCount`
  (params (Value :type Integer))
  (set `self.Count` Value))

(fn `UserConstructionScript`)